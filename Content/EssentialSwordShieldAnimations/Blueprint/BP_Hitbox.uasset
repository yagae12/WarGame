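; BP_Hitbox is an actor that hurts BP_Player on overlap, passing its location and AttackType as the damage position and hurt type.
; Its construction script colors the hitbox with a light or heavy material according to AttackType.
; After a hit, it disables collision and hides the mesh, then restores both after short delays, re-enabling collision last.
; A separate Box overlap with BP_Sword only prints a debug message.
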(event OnComponentBeginOverlap(Box)
  (params (OverlappedComponent :type Primitive%20Component%20Object%20Reference) (OtherActor :type Actor%20Object%20Reference) (OtherComp :type Primitive%20Component%20Object%20Reference) (OtherBodyIndex :type Integer) (bFromSweep :type Boolean) (SweepResult :type Hit%20Result%20Structure%20%28by%20ref%29))
  (Utilities|Casting|CastToBP_Sword OtherActor)
  (Development|PrintString "Hello"))

(event Collision|EventActorBeginOverlap
  (params (OtherActor :type Actor%20Object%20Reference))
  (bind _asbp_player (Utilities|Casting|CastToBP_Player OtherActor))
  (Default|Hurt _asbp_player (Transformation|GetActorLocation) (Variables|Default|GetAttackType))
  (Development|PrintString "Hit")
  (Collision|SetActorEnableCollision false)
  (Rendering|SetVisibility (Variables|Default|GetHitbox) false false)
  (Utilities|FlowControl|Delay 2.0)
  (Rendering|SetVisibility (Variables|Default|GetHitbox) true false)
  (Utilities|FlowControl|Delay 0.1)
  (Collision|SetActorEnableCollision true))

(fn ConstructionScript
  (bind _hitbox (Variables|Default|GetHitbox))
  (if (== (Variables|Default|GetAttackType) 0)
    (Rendering|Material|SetMaterial _hitbox 0 "/Game/EssentialSwordShieldAnimations/Material/MI_Hitbox_Light.MI_Hitbox_Light")
    (else
      (Rendering|Material|SetMaterial _hitbox 0 "/Game/EssentialSwordShieldAnimations/Material/MI_Hitbox_Heavy.MI_Hitbox_Heavy"))))